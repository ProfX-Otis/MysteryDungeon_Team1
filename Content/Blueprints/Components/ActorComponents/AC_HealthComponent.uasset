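; Actor component that tracks health for BP_ExplorerCharacter, caching its owner as that character on BeginPlay.
; Heal and TakeDamage adjust CurrentHealth, then call CheckHealth.
; CheckHealth clamps health at the maximum and zero, sets a status string by threshold, and calls the owner's PlayerDeathSequence at zero or below.
; Health from half up to three quarters of maximum matches no branch, leaving the previous status text.
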(event EventBeginPlay
  (bind _asbp_explorer_character (Utilities|Casting|CastToBP_ExplorerCharacter (Components|GetOwner)))
  (Variables|Default|SetPlayer_Ref _asbp_explorer_character))

(event EventTick
  (params (DeltaSeconds :type Float%20%28single-precision%29)))

(fn CheckHealth
  (if (>= (Variables|Default|GetCurrentHealth) (Variables|Default|GetMaxHealth))
    (Variables|Default|SetHealthStatus "Full Health :)")
    (Variables|Default|SetCurrentHealth (Variables|Default|GetMaxHealth))
    (elif (>= (Variables|Default|GetCurrentHealth) (* (Variables|Default|GetMaxHealth) 0.75))
      (Variables|Default|SetHealthStatus "Health Is Good!")
      (elif (and (< (Variables|Default|GetCurrentHealth) (* (Variables|Default|GetMaxHealth) 0.5)) (> (Variables|Default|GetCurrentHealth) 0.0))
        (Variables|Default|SetHealthStatus "Health Is Low!")
        (elif (<= (Variables|Default|GetCurrentHealth) 0.0)
          (Variables|Default|SetHealthStatus "You Are Dead!")
          (Variables|Default|SetCurrentHealth 0.0)
          (Default|PlayerDeathSequence (Variables|Default|GetPlayer_Ref)))))))

(fn Heal
  (params (HealAmount :type Float%20%28double-precision%29))
  (Variables|Default|SetCurrentHealth (+ HealAmount (Variables|Default|GetCurrentHealth)))
  (CallFunction|CheckHealth))

(fn TakeDamage
  (params (DamageAmount :type Float%20%28double-precision%29))
  (Variables|Default|SetCurrentHealth (- (Variables|Default|GetCurrentHealth) DamageAmount))
  (CallFunction|CheckHealth))