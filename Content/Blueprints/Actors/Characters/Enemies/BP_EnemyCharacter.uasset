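; Enemy character that patrols a looping list of target actors through its AI controller.
; BeginPlay binds the controller's move-completed event, and every result except Aborted triggers the next leg.
; Each leg waits a pause time, resets the detection light to patrol color and speed to walking, then moves to the next valid target.
; An incrementing index wrapped by modulo cycles the route.
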(event Custom|InitializePatrol
  (EventDispatchers|BindEventtoReceiveMoveCompleted (AI|GetAIController self) (delegate Custom|MoveComplete))
  (Utilities|MovetoNextTarget))

(event Custom|MoveComplete
  (params (RequestID :type AI%20Request%20ID%20Structure) (Result :type EPathFollowingResult%20Enum :default "Success"))
  (switch Utilities|FlowControl|Switch|SwitchonEPathFollowingResult Result
    (:Success
      _)
    (:Blocked
      _)
    (:OffPath
      _)
    (:Invalid
      _))
  (Utilities|MovetoNextTarget))

(event EventBeginPlay
  (CallFunction|InitializePatrol))

(fn ConstructionScript)

(fn InitizlizeDetection
  (Rendering|Components|Light|SetLightColor (Variables|Default|GetDetectionLight) (Variables|Default|GetPatrolColor) true)
  (Variables|/Script/Engine.CharacterMovementComponent|SetMaxWalkSpeed (Variables|Character|GetCharacterMovement) (Variables|Default|GetWalkSpeed)))

(fn LocateTargetMove
  (bind _self self)
  (bind _patroltargets (Variables|Default|GetPatrolTargets))
  (bind _returnvalue (AI|GetAIController _self))
  (bind _result (Math|Integer|IncrementInt (Variables|Default|GetPatrolTargetIndex))
    (:%20%20
      (Utilities|IsValid (Utilities|Array|Get(acopy) _patroltargets (Math|Integer|%(Integer) _result (Utilities|Array|Length _patroltargets)))
        (:Is%20Valid
          (Utilities|IsValid _returnvalue
            (:Is%20Valid
              (AI|Navigation|MovetoActor _returnvalue (Utilities|Array|Get(acopy) _patroltargets (Math|Integer|%(Integer) _result (Utilities|Array|Length _patroltargets))) -1.0 true true true 0))))))))