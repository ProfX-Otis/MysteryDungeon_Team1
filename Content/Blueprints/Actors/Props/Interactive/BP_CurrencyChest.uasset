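; BP_CurrencyChest is an interactive prop chest that gives currency to the explorer character.
; Overlapping the interact volume stores the player and toggles their prompt; the first interact swings the lid open by timeline, the next grants currency, hides the coins and destroys the volume.
; ResetChest respawns a fresh copy in place and destroys itself.
; A construction-script debug helper, marked for deletion before shipping, makes the interact volume visible in game.
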(event OnComponentBeginOverlap(ChestInteract)
  (params (OverlappedComponent :type Primitive%20Component%20Object%20Reference) (OtherActor :type Actor%20Object%20Reference) (OtherComp :type Primitive%20Component%20Object%20Reference) (OtherBodyIndex :type Integer) (bFromSweep :type Boolean) (SweepResult :type Hit%20Result%20Structure%20%28by%20ref%29))
  (bind _asbp_explorer_character (Utilities|Casting|CastToBP_ExplorerCharacter OtherActor))
  (bind _output_get (Variables|Default|SetPlayerRef _asbp_explorer_character))
  (Default|InteractTexton _output_get))

(event OnComponentEndOverlap(ChestInteract)
  (params (OverlappedComponent :type Primitive%20Component%20Object%20Reference) (OtherActor :type Actor%20Object%20Reference) (OtherComp :type Primitive%20Component%20Object%20Reference) (OtherBodyIndex :type Integer))
  (bind _asbp_explorer_character (Utilities|Casting|CastToBP_ExplorerCharacter OtherActor))
  (Default|InteractTextOff _asbp_explorer_character))

(event Custom|ResetChest
  (Game|SpawnActorfromClass "BP_CurrencyChest_C" (Transformation|GetActorTransform self) "Undefined" "MultiplyWithRoot" 0 0)
  (Actor|DestroyActor))

(event EventInteractIF
  (bind _playerref (Variables|Default|GetPlayerRef))
  (if (Variables|Default|GetChestOpen?)
    (Components|DestroyComponent (Variables|Default|GetChestInteract))
    (Variables|/Game/Blueprints/Actors/Characters/Players/BP_ExplorerCharacter.BP_ExplorerCharacter_C|SetCurrency _playerref (+ (Variables|/Game/Blueprints/Actors/Characters/Players/BP_ExplorerCharacter.BP_ExplorerCharacter_C|GetCurrency _playerref) 100))
    (Rendering|SetVisibility (Variables|Default|GetSM_ChestCoins_01a) false false)
    (else
      (Default|InteractTextOff (Variables|Default|GetPlayerRef))
      (Variables|Default|SetChestOpen? true)
      (bind _open_close (Timeline|Chest%20Anim PlayFromStart)
        (:Update
          (Transformation|SetRelativeRotation (Variables|Default|GetSM_OrnateChest_01d) (Math|Rotator|MakeRotator _open_close 0.0 0.0) false false)
          (Default|InteractTexton (Variables|Default|GetPlayerRef)))))))

(fn ConstructionScript
  (CallFunction|DELETEBEFORESHIPPING))

(fn DELETEBEFORESHIPPING
  (Development|SetHiddeninGame (Variables|Default|GetChestInteract) false false))