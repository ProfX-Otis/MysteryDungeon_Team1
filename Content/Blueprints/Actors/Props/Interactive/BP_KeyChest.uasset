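; Interactive key chest prop that shows an interact prompt while BP_ExplorerCharacter overlaps its trigger.
; The first interact plays timelines that swing the lid open, then bob and spin the revealed item.
; A second interact hides the item, increments the player's key count and destroys the trigger.
; ResetChest spawns an actor in its place and destroys itself; the construction script unhides the trigger in game as a pre-ship debug aid.
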(event OnComponentBeginOverlap(ChestInteract)
  (params (OverlappedComponent :type Primitive%20Component%20Object%20Reference) (OtherActor :type Actor%20Object%20Reference) (OtherComp :type Primitive%20Component%20Object%20Reference) (OtherBodyIndex :type Integer) (bFromSweep :type Boolean) (SweepResult :type Hit%20Result%20Structure%20%28by%20ref%29))
  (bind _asbp_explorer_character (Utilities|Casting|CastToBP_ExplorerCharacter OtherActor))
  (bind _output_get (Variables|Default|SetPlayerRef _asbp_explorer_character))
  (Default|InteractTexton _output_get))

(event OnComponentEndOverlap(ChestInteract)
  (params (OverlappedComponent :type Primitive%20Component%20Object%20Reference) (OtherActor :type Actor%20Object%20Reference) (OtherComp :type Primitive%20Component%20Object%20Reference) (OtherBodyIndex :type Integer))
  (bind _asbp_explorer_character (Utilities|Casting|CastToBP_ExplorerCharacter OtherActor))
  (Default|InteractTextOff _asbp_explorer_character))

(event Custom|ResetChest
  (Game|SpawnActorfromClass "BP_KeyChest_C" (Transformation|GetActorTransform self) "Undefined" "MultiplyWithRoot" 0 0)
  (Actor|DestroyActor))

(event EventInteractIF
  (bind _item (Variables|Default|GetItem))
  (bind _playerref (Variables|Default|GetPlayerRef))
  (if (Variables|Default|GetChestOpen?)
    (Rendering|SetVisibility _item false false)
    (Components|DestroyComponent (Variables|Default|GetChestInteract))
    (Variables|/Game/Blueprints/Actors/Characters/Players/BP_ExplorerCharacter.BP_ExplorerCharacter_C|SetKeys _playerref (+ (Variables|/Game/Blueprints/Actors/Characters/Players/BP_ExplorerCharacter.BP_ExplorerCharacter_C|GetKeys _playerref) 1))
    (else
      (Default|InteractTextOff (Variables|Default|GetPlayerRef))
      (Rendering|SetVisibility _item true false)
      (Variables|Default|SetChestOpen? true)
      (bind (_direction _open_close _itemlocation _itemrotation) (Timeline|ChestAnim Play)
        (:Update
          (Transformation|SetRelativeRotation (Variables|Default|GetSM_OrnateChest_01d) (Math|Rotator|MakeRotator _open_close 0.0 0.0) false false)
          (Transformation|SetRelativeLocationAndRotation (Variables|Default|GetItemOffset) (Math|Vector|MakeVector 0.0 0.0 _itemlocation) (Math|Rotator|MakeRotator 0.0 0.0 _itemrotation) false false))
        (:Finished
          (bind (_direction_2 _bob _spin) (Timeline|IdleAnim Play)
            (:Update
              (Transformation|SetRelativeLocationAndRotation (Variables|Default|GetItemOffset) (Math|Vector|MakeVector 0.0 0.0 _bob) (Math|Rotator|MakeRotator 0.0 0.0 _spin) false false)
              (Default|InteractTexton (Variables|Default|GetPlayerRef)))))))))

(fn ConstructionScript
  (CallFunction|DELETEBEFORESHIPPING))

(fn DELETEBEFORESHIPPING
  (Development|SetHiddeninGame (Variables|Default|GetChestInteract) false false))