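; Trap chest prop that the explorer character opens through an interact event, revealing a bomb and briefly spawning a damage item.
; Overlapping the trigger toggles the player's prompt; interacting removes the trigger and runs a timeline rotating the lid and moving the bomb offset.
; When finished, it hides the bomb and spawns a hidden BP_DamageItem, destroyed shortly after.
; ResetChest replaces the actor with a fresh copy; a construction-script debug function unhides the trigger.
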(event OnComponentBeginOverlap(ChestInteract)
  (params (OverlappedComponent :type Primitive%20Component%20Object%20Reference) (OtherActor :type Actor%20Object%20Reference) (OtherComp :type Primitive%20Component%20Object%20Reference) (OtherBodyIndex :type Integer) (bFromSweep :type Boolean) (SweepResult :type Hit%20Result%20Structure%20%28by%20ref%29))
  (bind _asbp_explorer_character (Utilities|Casting|CastToBP_ExplorerCharacter OtherActor))
  (bind _output_get (Variables|Default|SetPlayerRef _asbp_explorer_character))
  (Default|InteractTexton _output_get))

(event OnComponentEndOverlap(ChestInteract)
  (params (OverlappedComponent :type Primitive%20Component%20Object%20Reference) (OtherActor :type Actor%20Object%20Reference) (OtherComp :type Primitive%20Component%20Object%20Reference) (OtherBodyIndex :type Integer))
  (bind _asbp_explorer_character (Utilities|Casting|CastToBP_ExplorerCharacter OtherActor))
  (Default|InteractTextOff _asbp_explorer_character))

(event Custom|ResetChest
  (Game|SpawnActorfromClass "BP_TrapChest_C" (Transformation|GetActorTransform self) "Undefined" "MultiplyWithRoot" 0 0)
  (Actor|DestroyActor))

(event EventInteractIF
  (Default|InteractTextOff (Variables|Default|GetPlayerRef))
  (Components|DestroyComponent (Variables|Default|GetChestInteract))
  (bind (_direction _open_close _itemlocation _itemrotation) (Timeline|ChestAnim PlayFromStart)
    (:Update
      (Transformation|SetRelativeRotation (Variables|Default|GetSM_OrnateChest_01d) (Math|Rotator|MakeRotator _open_close 0.0 0.0) false false)
      (Transformation|SetRelativeLocationAndRotation (Variables|Default|GetItemOffset) (Math|Vector|MakeVector 0.0 0.0 _itemlocation) (Math|Rotator|MakeRotator 0.0 0.0 _itemrotation) false false)
      (Default|InteractTextOff (Variables|Default|GetPlayerRef)))
    (:Finished
      (Rendering|SetVisibility (Variables|Default|GetBomb) false false)
      (bind _returnvalue (Game|SpawnActorfromClass "/Game/Blueprints/Actors/Items/Collectables/Health/BP_DamageItem.BP_DamageItem_C" (Transformation|GetActorTransform self) "Undefined" "MultiplyWithRoot" 0 0))
      (Utilities|IsValid _returnvalue
        (:Is%20Valid
          (Rendering|SetActorHiddenInGame _returnvalue true)
          (Utilities|FlowControl|Delay 0.1)
          (Utilities|IsValid _returnvalue
            (:Is%20Valid
              (Actor|DestroyActor _returnvalue))))))))

(fn ConstructionScript
  (CallFunction|DELETEBEFORESHIPPING))

(fn DELETEBEFORESHIPPING
  (Development|SetHiddeninGame (Variables|Default|GetChestInteract) false false))