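; BP_NextLevelZone is a level exit trigger that sends the explorer to a named level once they hold enough keys.
; On overlap, it checks the explorer's keys against a requirement, pushes currency, keys and health to the mystery dungeon GameInstance to persist them, then opens the level.
; Too few keys only prints a debug refusal message.
; The construction script makes the collider visible in game via a function marked for removal before shipping.
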(event OnComponentBeginOverlap(NextLevelCollider)
  (params (OverlappedComponent :type Primitive%20Component%20Object%20Reference) (OtherActor :type Actor%20Object%20Reference) (OtherComp :type Primitive%20Component%20Object%20Reference) (OtherBodyIndex :type Integer) (bFromSweep :type Boolean) (SweepResult :type Hit%20Result%20Structure%20%28by%20ref%29))
  (bind _asbp_explorer_character (Utilities|Casting|CastToBP_ExplorerCharacter OtherActor))
  (if (>= (Variables|/Game/Blueprints/Actors/Characters/Players/BP_ExplorerCharacter.BP_ExplorerCharacter_C|GetKeys _asbp_explorer_character) (Variables|Default|GetKeysRequirement))
    (Default|PushVariables (Variables|Default|GetGI_Ref) (Variables|/Game/Blueprints/Actors/Characters/Players/BP_ExplorerCharacter.BP_ExplorerCharacter_C|GetCurrency _asbp_explorer_character) (Variables|/Game/Blueprints/Actors/Characters/Players/BP_ExplorerCharacter.BP_ExplorerCharacter_C|GetKeys _asbp_explorer_character) (Variables|/Game/Blueprints/Components/ActorComponents/AC_HealthComponent.AC_HealthComponent_C|GetCurrentHealth (Variables|/Game/Blueprints/Actors/Characters/Players/BP_ExplorerCharacter.BP_ExplorerCharacter_C|GetAC_HealthComponent _asbp_explorer_character)))
    (Game|OpenLevel(byName) (Variables|Default|GetLevel%20Name))
    (else
      (Development|PrintString "YOU SHALL NOT PASS"))))

(event EventBeginPlay
  (bind _asbp_mystery_dungeon_gi (Utilities|Casting|CastToBP_MysteryDungeon_GI (Game|GetGameInstance)))
  (Variables|Default|SetGI_Ref _asbp_mystery_dungeon_gi))

(fn ConstructionScript
  (CallFunction|DElETEBEFORESHIPPING))

(fn DElETEBEFORESHIPPING
  (Development|SetHiddeninGame (Variables|Default|GetNextLevelCollider) false false))