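; BP_HealthOverTimeAOE is an area-of-effect zone that heals a BP_ExplorerCharacter over time while it overlaps the HealthZone component.
; On overlap begin it stores the character and starts healing through that character's health component.
; StartHealing re-arms a one-second timer on itself to repeat each heal.
; On overlap end it clears the stored reference and invalidates the timer.
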(event OnComponentBeginOverlap(HealthZone)
  (params (OverlappedComponent :type Primitive%20Component%20Object%20Reference) (OtherActor :type Actor%20Object%20Reference) (OtherComp :type Primitive%20Component%20Object%20Reference) (OtherBodyIndex :type Integer) (bFromSweep :type Boolean) (SweepResult :type Hit%20Result%20Structure%20%28by%20ref%29))
  (bind _asbp_explorer_character (Utilities|Casting|CastToBP_ExplorerCharacter OtherActor))
  (Variables|Default|SetPlayerRef _asbp_explorer_character)
  (CallFunction|StartHealing))

(event OnComponentEndOverlap(HealthZone)
  (params (OverlappedComponent :type Primitive%20Component%20Object%20Reference) (OtherActor :type Actor%20Object%20Reference) (OtherComp :type Primitive%20Component%20Object%20Reference) (OtherBodyIndex :type Integer))
  (Utilities|Casting|CastToBP_ExplorerCharacter OtherActor)
  (Variables|Default|SetPlayerRef 0)
  (CallFunction|StopHealing))

(event Custom|StartHealing
  (bind _returnvalue (Utilities|Time|SetTimerbyEvent (delegate Custom|StartHealing) 1.0))
  (Default|Heal (Variables|/Game/Blueprints/Actors/Characters/Players/BP_ExplorerCharacter.BP_ExplorerCharacter_C|GetAC_HealthComponent (Variables|Default|GetPlayerRef)) 1e+01))

(event Custom|StopHealing
  (Utilities|Time|ClearandInvalidateTimerbyHandle (stale Custom|StartHealing _returnvalue)))

(fn ConstructionScript)