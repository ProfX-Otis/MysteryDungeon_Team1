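; Area-of-effect hazard actor that deals damage over time to the player while they stand inside it.
; The HealthZone overlap component stores the entering BP_ExplorerCharacter and applies fixed damage immediately through its ACHealthComponent.
; StartDamage re-schedules itself with a one-second timer to repeat the damage.
; Leaving the zone clears the player reference and invalidates the timer.
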(event OnComponentBeginOverlap(HealthZone)
  (params (OverlappedComponent :type Primitive%20Component%20Object%20Reference) (OtherActor :type Actor%20Object%20Reference) (OtherComp :type Primitive%20Component%20Object%20Reference) (OtherBodyIndex :type Integer) (bFromSweep :type Boolean) (SweepResult :type Hit%20Result%20Structure%20%28by%20ref%29))
  (bind _asbp_explorer_character (Utilities|Casting|CastToBP_ExplorerCharacter OtherActor))
  (Variables|Default|SetPlayerRef _asbp_explorer_character)
  (CallFunction|StartDamage))

(event OnComponentEndOverlap(HealthZone)
  (params (OverlappedComponent :type Primitive%20Component%20Object%20Reference) (OtherActor :type Actor%20Object%20Reference) (OtherComp :type Primitive%20Component%20Object%20Reference) (OtherBodyIndex :type Integer))
  (Utilities|Casting|CastToBP_ExplorerCharacter OtherActor)
  (Variables|Default|SetPlayerRef 0)
  (CallFunction|StopDamage))

(event Custom|StartDamage
  (bind _returnvalue (Utilities|Time|SetTimerbyEvent (delegate Custom|StartDamage) 1.0))
  (Default|TakeDamage (Variables|/Game/Blueprints/Actors/Characters/Players/BP_ExplorerCharacter.BP_ExplorerCharacter_C|GetAC_HealthComponent (Variables|Default|GetPlayerRef)) 5.0))

(event Custom|StopDamage
  (Utilities|Time|ClearandInvalidateTimerbyHandle (stale Custom|StartDamage _returnvalue)))

(fn ConstructionScript)